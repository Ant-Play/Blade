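; Player character with crouch, sprint, vaulting and stealth assassination, plus a center-point HUD widget.
; Crouch and sprint adjust walk speed alongside camera distance or mode, with sprint release restoring the volume or default camera mode.
; Vault traces find start, middle and landing points, then drive a motion-warped montage in flying mode without collision.
; Assassination queries overlapping BPI_Assasination actors for a warp target and plays the attacker's paired knife montage.
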(event Custom|VaultMotionWarping
  (bind _mesh (Variables|Character|GetMesh))
  (bind _returnvalue (Transformation|GetWorldLocation _mesh))
  ;[1 1 1] VaultMotionWarp
  (if (and (Variables|Vault|GetbMotionWarp) (Math|Float|InRange(Float) (.z (Variables|Vault|GetVaultLandPos)) (- (.z _returnvalue) 5e+01) (+ (.z _returnvalue) 5e+01)))
    (Pawn|Components|CharacterMovement|SetMovementMode (Variables|Character|GetCharacterMovement) "MOVE_Flying" 0)
    (Collision|SetActorEnableCollision false)
    (Class|MotionWarpingComponent|AddorUpdateWarpTarget (Variables|Default|GetMotionWarping) (Utilities|Struct|MakeMotionWarpingTarget "VaultStart" (Variables|Vault|GetVaultStartPos) (Transformation|GetActorRotation) 0 "None" false))
    (Class|MotionWarpingComponent|AddorUpdateWarpTarget (Variables|Default|GetMotionWarping) (Utilities|Struct|MakeMotionWarpingTarget "VaultMiddle" (Variables|Vault|GetVaultMiddlePos) (Transformation|GetActorRotation) 0 "None" false))
    (Class|MotionWarpingComponent|AddorUpdateWarpTarget (Variables|Default|GetMotionWarping) (Utilities|Struct|MakeMotionWarpingTarget "VaultLand" (Variables|Vault|GetVaultLandPos) (Transformation|GetActorRotation) 0 "None" false))
    (Animation|Montage|PlayMontage (Variables|Character|GetMesh) "/Game/Characters/Blade_Character/Animation/Vault/VaultOver_Montage.VaultOver_Montage"
      (:OnCompleted
        (Pawn|Components|CharacterMovement|SetMovementMode (Variables|Character|GetCharacterMovement) "MOVE_Walking" 0)
        (Collision|SetActorEnableCollision true)
        (Variables|Vault|SetbMotionWarp false)
        (Variables|Vault|SetVaultLandPos "0.000000,0.000000,20000.000000")))))

(event Custom|Crouch/Uncrouch
  (bind _cameracomponent (Variables|Default|GetCameraComponent))
  (bind _charactermovement (Variables|Character|GetCharacterMovement))
  (bind _oldcameradistance (Variables|Default|GetOldCameraDistance))
  ;[1 1 1] ChrouchAction
  (if (not (Variables|Default|GetChrouched))
    (Variables|Default|SetChrouched true)
    (Variables|/Script/Engine.CharacterMovementComponent|SetMaxWalkSpeed _charactermovement 3.5e+02)
    (Class|ATPCCameraComponent|SetCameraDistance _cameracomponent (+ _oldcameradistance 1.5e+02) true)
    (else
      (Variables|Default|SetChrouched false)
      (Variables|/Script/Engine.CharacterMovementComponent|SetMaxWalkSpeed _charactermovement 5e+02)
      (Class|ATPCCameraComponent|SetCameraDistance _cameracomponent _oldcameradistance true))))

(event Input|EnhancedActionEvents|EnhancedInputActionIA_Crouch
  (params (ActionValue :type Boolean) (ElapsedSeconds :type Float%20%28double-precision%29) (TriggeredSeconds :type Float%20%28double-precision%29) (InputAction :type Input%20Action%20Object%20Reference :default "/Game/Inputs/Actions/IA_Crouch.IA_Crouch"))
  (bind _cameracomponent (Variables|Default|GetCameraComponent))
  (bind _charactermovement (Variables|Character|GetCharacterMovement))
  (bind _oldcameradistance (Variables|Default|GetOldCameraDistance))
  ;[1 1 1] ChrouchAction
  (:Started
    (if (not (Variables|Default|GetChrouched))
      (Variables|Default|SetChrouched true)
      (Variables|/Script/Engine.CharacterMovementComponent|SetMaxWalkSpeed _charactermovement 3.5e+02)
      (Class|ATPCCameraComponent|SetCameraDistance _cameracomponent (+ _oldcameradistance 1.5e+02) true)
      (else
        (Variables|Default|SetChrouched false)
        (Variables|/Script/Engine.CharacterMovementComponent|SetMaxWalkSpeed _charactermovement 5e+02)
        (Class|ATPCCameraComponent|SetCameraDistance _cameracomponent _oldcameradistance true)))))

(event Input|EnhancedActionEvents|EnhancedInputActionIA_Vault
  (params (ActionValue :type Boolean) (ElapsedSeconds :type Float%20%28double-precision%29) (TriggeredSeconds :type Float%20%28double-precision%29) (InputAction :type Input%20Action%20Object%20Reference :default "/Game/Inputs/Actions/IA_Vault.IA_Vault"))
  ;[1 1 1] VaultMotionWarp
  (:Started
    (CallFunction|Vault)))

(event Input|EnhancedActionEvents|EnhancedInputActionIA_Sprits
  (params (ActionValue :type Boolean) (ElapsedSeconds :type Float%20%28double-precision%29) (TriggeredSeconds :type Float%20%28double-precision%29) (InputAction :type Input%20Action%20Object%20Reference :default "/Game/Inputs/Actions/IA_Sprits.IA_Sprits"))
  (bind _charactermovement (Variables|Character|GetCharacterMovement))
  ;[1 1 1] Spirts
  (:Started
    (Class|ATPCCameraComponent|SetCameraMode (Variables|Default|GetCameraComponent) "(TagName=\"CameraMode.Sprint\")" true false)
    (Variables|/Script/Engine.CharacterMovementComponent|SetMaxWalkSpeed _charactermovement 9e+02))
  (:Completed
    (CallFunction|SetDefaultorVolumeCameraMode)
    (Variables|/Script/Engine.CharacterMovementComponent|SetMaxWalkSpeed _charactermovement 5e+02)))

(event Input|EnhancedActionEvents|EnhancedInputActionIA_Assasination
  (params (ActionValue :type Boolean) (ElapsedSeconds :type Float%20%28double-precision%29) (TriggeredSeconds :type Float%20%28double-precision%29) (InputAction :type Input%20Action%20Object%20Reference :default "/Game/Inputs/Actions/IA_Assasination.IA_Assasination"))
  ;[1 1 1] Stealth Assasination
  (:Started
    (for _array_element (Collision|GetOverlappingActors 0 :!class /Script/Engine.Actor)
      (if (Utilities|DoesObjectImplementInterface _array_element "/Game/Blueprint/BPI_Assasination.BPI_Assasination_C")
        (bind (_ref_location _assasin_rotation) (Class|BPIAssasination|StealthBackAssasin(Message) _array_element))
        (Animation|Montage|PlayMontage (Variables|Character|GetMesh) "/Game/Characters/Blade_Character/Animation/Assasinations/Paired_Knife_Stealth_KidneyAndNeck_Att_Montage.Paired_Knife_Stealth_KidneyAndNeck_Att_Montage"
          (:then
            (Class|MotionWarpingComponent|AddorUpdateWarpTarget (Variables|Default|GetMotionWarping) (Utilities|Struct|MakeMotionWarpingTarget "AssasinationWarp" _ref_location _assasin_rotation 0 "None" false))))))))

(event EventBeginPlay
  ;[1 1 1] WindowCenterPoint
  (|CallParentFunction)
  (bind _returnvalue (UserInterface|CreateWidget "/Game/UI/WB_MiddlePoint.WB_MiddlePoint_C"))
  (UserInterface|Viewport|AddtoViewport _returnvalue 0)
  (Variables|Default|SetOldCameraDistance (Class|ATPCCameraComponent|GetCameraDistance (Variables|Default|GetCameraComponent))))

(event Collision|EventActorBeginOverlap
  (params (OtherActor :type Actor%20Object%20Reference)))

(event EventTick
  (params (DeltaSeconds :type Float%20%28single-precision%29)))

(event Input|KeyboardEvents|SpaceBar
  (params (Key :type Key%20Structure :default "None"))
  ;[1 1 1] ChrouchAction
  (:Pressed
    (if (Variables|Default|GetChrouched)
      (CallFunction|Crouch/Uncrouch))))

(fn ConstructionScript)

(fn Vault
  (bind _index (Utilities|FlowControl|ForLoopwithBreak 0 2 :!label _label)
    (:LoopBody
      (bind (_outhit _returnvalue) (Collision|SphereTraceByChannel (+ (Transformation|GetActorLocation) (Math|Vector|MakeVector 0.0 0.0 (* _index 3e+01))) (+ (+ (Transformation|GetActorLocation) (Math|Vector|MakeVector 0.0 0.0 (* _index 3e+01))) (* (Math|Vector|GetForwardVector (Transformation|GetActorRotation)) 1.8e+02)) 5.0 "TraceTypeQuery1" false 0 "ForDuration"))
      (if _returnvalue
        (Utilities|FlowControl|Sequence
          (:then_0
            (goto _label Break))
          (:then_1
            (bind _index_2 (Utilities|FlowControl|ForLoopwithBreak 0 5 :!label _label_2)
              (:LoopBody
                (bind (_outhit_2 _returnvalue_2) (Collision|SphereTraceByChannel (+ (+ (.Location (Collision|BreakHitResult _outhit)) "0.000000,0.000000,100.000000") (* (Math|Vector|GetForwardVector (Transformation|GetActorRotation)) (* _index_2 5e+01))) (- (+ (+ (.Location (Collision|BreakHitResult _outhit)) "0.000000,0.000000,100.000000") (* (Math|Vector|GetForwardVector (Transformation|GetActorRotation)) (* _index_2 5e+01))) "0.000000,0.000000,100.000000") 1e+01 "TraceTypeQuery1" false 0 "None"))
                (if _returnvalue_2
                  (Utilities|FlowControl|Sequence
                    (:then_0
                      (if (== _index_2 0)
                        (bind _output_get (Variables|Vault|SetVaultStartPos (.Location (Collision|BreakHitResult _outhit_2))))
                        (Rendering|Debug|DrawDebugSphere _output_get 1e+01 12 "(R=1.000000,G=0.118343,B=0.845300,A=1.000000)" 1e+01 2.0)))
                    (:then_1
                      (bind _output_get_2 (Variables|Vault|SetVaultMiddlePos (.Location (Collision|BreakHitResult _outhit_2))))
                      (Rendering|Debug|DrawDebugSphere _output_get_2 1e+01 12 "(R=1.000000,G=0.950883,B=0.066792,A=1.000000)" 1e+01 2.0)
                      (Variables|Vault|SetbMotionWarp true)))
                  (else
                    (bind (_outhit_3 _returnvalue_3) (Collision|LineTraceByChannel (+ (.TraceStart (Collision|BreakHitResult _outhit_2)) (* (Math|Vector|GetForwardVector (Transformation|GetActorRotation)) 8e+01)) (- (+ (.TraceStart (Collision|BreakHitResult _outhit_2)) (* (Math|Vector|GetForwardVector (Transformation|GetActorRotation)) 8e+01)) "0.000000,0.000000,1000.000000") "TraceTypeQuery1" false 0 "ForDuration" true "(R=0.104009,G=0.054318,B=1.000000,A=1.000000)"))
                    (if _returnvalue_3
                      (Variables|Vault|SetVaultLandPos (.Location (Collision|BreakHitResult _outhit_3)))
                      (goto _label_2 Break)))))
              (:Completed
                (CallFunction|VaultMotionWarping)))))))))

(fn SetDefaultorVolumeCameraMode
  (bind _cameracomponent (Variables|Default|GetCameraComponent))
  (bind _returnvalue (Class|ATPCCameraComponent|GetCameraModeTagfromOverlapCameraVolume _cameracomponent))
  (Class|ATPCCameraComponent|SetCameraMode _cameracomponent (select (GameplayTags|IsGameplayTagValid _returnvalue) _returnvalue (Variables|/Script/ThirdPersonCamera.ATPCCameraComponent|GetDefaultCameraModeTag _cameracomponent)) true false))