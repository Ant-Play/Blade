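; BP_Dummy is a target character that MainCharacter can stealth-assassinate from behind.
; An AssasinationRadius overlap shows or hides the AssasinateWidget prompt, which starts hidden.
; StealthBackAssasin plays the victim half of a paired knife montage, triggers a delayed mesh ragdoll, hides the prompt, and returns the AssasinREF transform, presumably to align the attacker.
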(event OnComponentBeginOverlap(AssasinationRadius)
  (params (OverlappedComponent :type Primitive%20Component%20Object%20Reference) (OtherActor :type Actor%20Object%20Reference) (OtherComp :type Primitive%20Component%20Object%20Reference) (OtherBodyIndex :type Integer) (bFromSweep :type Boolean) (SweepResult :type Hit%20Result%20Structure%20%28by%20ref%29))
  (Utilities|Casting|CastToMainCharacter OtherActor)
  (Rendering|SetVisibility (Variables|Default|GetAssasinate%20Widget) true false))

(event OnComponentEndOverlap(AssasinationRadius)
  (params (OverlappedComponent :type Primitive%20Component%20Object%20Reference) (OtherActor :type Actor%20Object%20Reference) (OtherComp :type Primitive%20Component%20Object%20Reference) (OtherBodyIndex :type Integer))
  (Utilities|Casting|CastToMainCharacter OtherActor)
  (Rendering|SetVisibility (Variables|Default|GetAssasinate%20Widget) false false))

(event Custom|Ragdoll
  ;[1 1 1] Ragdoll
  (Utilities|FlowControl|Delay 2.5)
  (Physics|SetSimulatePhysics (Variables|Character|GetMesh) true))

(event EventBeginPlay
  (Rendering|SetVisibility (Variables|Default|GetAssasinate%20Widget) false false))

(event Collision|EventActorBeginOverlap
  (params (OtherActor :type Actor%20Object%20Reference)))

(event EventTick
  (params (DeltaSeconds :type Float%20%28single-precision%29)))

(fn ConstructionScript)

(fn StealthBackAssasin
  (bind _assasin_ref (Variables|Default|GetAssasin%20REF))
  (Animation|PlayAnimMontage "/Game/Characters/Blade_Character/Animation/Assasinations/Paired_Knife_Stealth_KidneyAndNeck_Vic_Montage.Paired_Knife_Stealth_KidneyAndNeck_Vic_Montage" 1.0 "None")
  (CallFunction|Ragdoll)
  (Rendering|SetVisibility (Variables|Default|GetAssasinate%20Widget) false false)
  (return (Transformation|GetWorldLocation _assasin_ref) (Transformation|GetWorldRotation _assasin_ref)))